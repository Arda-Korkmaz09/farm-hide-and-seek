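; BP_HaritaYoneticisi is a map manager that randomly populates a box volume with nests and decorations at BeginPlay.
; It force-spawns each YuvaListesi class once at a random point in the box.
; It then makes DekorasyonSayisi-driven attempts to place random DekorasyonListesi classes, spawning only if a WorldStatic sphere overlap finds nothing.
; That overlap has no position input, so it does not test the chosen point.
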(event EventBeginPlay
  (bind _box (Variables|Default|GetBox))
  (bind _box_2 (Variables|Default|GetBox))
  (bind _dekorasyonlistesi (Variables|Default|GetDekorasyonListesi))
  (bind (_origin _boxextent) (Collision|GetComponentBounds _box))
  (bind (_origin_2 _boxextent_2) (Collision|GetComponentBounds _box_2))
  (for _array_element (Variables|Default|GetYuvaListesi)
    (Game|SpawnActorfromClass _array_element (Math|Conversions|ToTransform(Vector) (Math|Random|RandomPointinBoundingBox _origin_2 _boxextent_2)) "AlwaysSpawn" "MultiplyWithRoot" 0 0))
  (for _index (range 0 (Variables|Default|GetDekorasyonSayisi))
    (bind _output_get (Variables|Default|SetGeciciKonum (Math|Random|RandomPointinBoundingBox _origin _boxextent)))
    (bind _outactors (Collision|SphereOverlapActors "0, 0, 0" 1e+02 (Utilities|Array|MakeArray "ObjectTypeQuery1") 0))
    (if (== (Utilities|Array|Length _outactors) 0)
      (Game|SpawnActorfromClass (Utilities|Array|Get(acopy) _dekorasyonlistesi (Math|Random|RandomIntegerinRange 0 (Utilities|Array|LastIndex _dekorasyonlistesi))) (Math|Conversions|ToTransform(Vector) _output_get) "Undefined" "MultiplyWithRoot" 0 0))))

(fn ConstructionScript)