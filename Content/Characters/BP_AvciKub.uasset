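; BP_AvciKub is a player-controlled hunter Character that moves, looks, jumps and shoots.
; Input axes and actions drive movement, mouse look and jumping, while the 1 key toggles visibility of the Nişangah (crosshair) component.
; Left click runs a debug-drawn Visibility line trace forward from Nişangah and applies damage to the hit actor.
; The destroy-on-hit branch is disconnected, and the Move and Aim functions are empty.
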(event Input|ActionEvents|InputActionziplama
  (params (Key :type Key%20Structure :default "None"))
  (:Pressed
    (Character|Jump))
  (:Released
    (Character|StopJumping)))

(event Input|AxisEvents|InputAxisilerigeri
  (params (AxisValue :type Float%20%28single-precision%29))
  (Pawn|Input|AddMovementInput (Transformation|GetActorForwardVector) AxisValue false))

(event Input|AxisEvents|InputAxissağsol
  (params (AxisValue :type Float%20%28single-precision%29))
  (Pawn|Input|AddMovementInput (Transformation|GetActorRightVector) AxisValue false))

(event Input|MouseEvents|MouseX
  (params (AxisValue :type Float%20%28single-precision%29))
  (Pawn|Input|AddControllerYawInput AxisValue))

(event Input|MouseEvents|MouseY
  (params (AxisValue :type Float%20%28single-precision%29))
  (Pawn|Input|AddControllerPitchInput (* AxisValue -1.0)))

(event Input|MouseEvents|LeftMouseButton
  (params (Key :type Key%20Structure :default "None"))
  (bind _nişangah (Variables|Default|Getnişangah))
  (bind _returnvalue (Transformation|GetWorldLocation _nişangah))
  (:Pressed
    (Development|PrintString "Ateş etti")
    (bind (_outhit _returnvalue_2) (Collision|LineTraceByChannel _returnvalue (+ _returnvalue (* (Math|Vector|GetForwardVector _nişangah) 2.5e+03)) "TraceTypeQuery1" false 0 "ForDuration"))
    (Game|Damage|ApplyDamage (.hitactor _outhit) 1.0 0 0)))

(event Input|KeyboardEvents|1
  (params (Key :type Key%20Structure :default "None"))
  (bind _nişangah (Variables|Default|Getnişangah))
  (:Pressed
    (Utilities|FlowControl|FlipFlop
      (:A
        (Rendering|SetVisibility _nişangah true false))
      (:B
        (Rendering|SetVisibility _nişangah false false)))))

(fn ConstructionScript)

(fn Move
  (params (X%20Axis :type Float%20%28double-precision%29) (Y%20Axis :type Float%20%28double-precision%29)))

(fn Aim
  (params (X%20Axis :type Float%20%28single-precision%29) (Y%20Axis :type Float%20%28double-precision%29)))